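; Hero gameplay ability that consumes one HP portion (potion) when activated.
; It casts the avatar to BaseHero, reads the portion count from the main widget and, if nonzero, writes back one less and removes a BP_HPPortion item from the inventory component.
; The widget's count gates use, the ability ends immediately either way, and the graph itself applies no healing.
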(event `self.K2_ActivateAbility`
  (bind (_returnvalue_owneractor _returnvalue_avataractor) (break `GameplayAbilityActorInfo` (`self.GetActorInfo`)))
  (bind _asbase_hero (cast `BaseHero` _returnvalue_avataractor))
  (bind _mainwidget (`BaseHero.MainWidget` _asbase_hero))
  (bind _returnvalue (`MainScreenWidget.GetHPPortion` _mainwidget))
  (if (!= _returnvalue 0)
    (`MainScreenWidget.SetHPPortion` _mainwidget (- _returnvalue 1))
    (`InventoryComponent.RemoveItem` (`BaseHero.InventoryComponent` _asbase_hero) "/Game/Blueprints/Items/BP_HPPortion.BP_HPPortion_C")
    (`self.K2_EndAbility`)
    (else
      (`self.K2_EndAbility`))))