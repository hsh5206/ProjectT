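; Hero gameplay ability for using an MP potion from the potion count shown on the main widget.
; On activation it decrements a nonzero MP count, removes a BP_HPPortion item (the HP class, not MP) from the inventory, and refreshes the MP bar from Mana and MaxMana.
; It applies no mana change or gameplay effect itself, and ends immediately on either branch.
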(event `self.K2_ActivateAbility`
  (bind (_returnvalue_owneractor _returnvalue_avataractor) (break `GameplayAbilityActorInfo` (`self.GetActorInfo`)))
  (bind _asbase_hero (cast `BaseHero` _returnvalue_avataractor))
  (bind _mainwidget (`BaseHero.MainWidget` _asbase_hero))
  (bind _returnvalue (`MainScreenWidget.GetMPPortion` _mainwidget))
  (if (!= _returnvalue 0)
    (`MainScreenWidget.SetMPPortion` _mainwidget (- _returnvalue 1))
    (`InventoryComponent.RemoveItem` (`BaseHero.InventoryComponent` _asbase_hero) "/Game/Blueprints/Items/BP_HPPortion.BP_HPPortion_C")
    (bind _attributes (`BaseCharacter.Attributes` _asbase_hero))
    (bind (_mana_basevalue _mana_currentvalue) (break `GameplayAttributeData` (`PTAttributeSet.Mana` _attributes)))
    (bind (_maxmana_basevalue _maxmana_currentvalue) (break `GameplayAttributeData` (`PTAttributeSet.MaxMana` _attributes)))
    (`MainScreenWidget.SetMPBarPercent` _mainwidget _mana_currentvalue _maxmana_currentvalue)
    (`self.K2_EndAbility`)
    (else
      (`self.K2_EndAbility`))))