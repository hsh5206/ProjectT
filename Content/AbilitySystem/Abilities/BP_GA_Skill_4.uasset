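; BP_GA_Skill_4 is a gameplay ability that plays a hero's fourth skill montage while letting the hero pass through pawns.
; After a tiny delay, only the authority ignores the capsule's Pawn channel and plays the montage; other instances end immediately.
; The SkillAttackEnd event stops the montage through ServerStopMontage, restores Pawn blocking and ends the ability.
; Normal montage completion also ends the ability but leaves collision unrestored.
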(event `self.K2_ActivateAbility`
  (bind (_returnvalue_owneractor _returnvalue_avataractor) (break `GameplayAbilityActorInfo` (`self.GetActorInfo`)))
  (bind _hero (`self.Hero`))
  (`KismetSystemLibrary.Delay` 0.01)
  (bind _asbase_hero (cast `BaseHero` (`self.GetAvatarActorFromActorInfo`)))
  (set `self.Hero` _asbase_hero)
  (if (`Actor.HasAuthority` _hero)
    (`PrimitiveComponent.SetCollisionResponseToChannel` (`Character.CapsuleComponent` _hero) "ECC_Pawn" "ECR_Ignore")
    ;[1 1 1] PlayMontage
    (`AT_PlayMontageAndWaitForEvent.PlayMontageAndWaitForEvent` "None" "/Game/Blueprints/Characters/Hero/Animations/AM_SKill_4.AM_SKill_4" (struct :`GameplayTags` (struct :`(TagName` "Event.Attack.SkillAttackEnd")))
      (:`OnCompleted`
        _)
      (:`EventReceived`
        (bind _asbase_character (cast `BaseCharacter` _returnvalue_avataractor))
        (`BaseCharacter.ServerStopMontage` _asbase_character "/Game/Blueprints/Characters/Hero/Animations/AM_SKill_4.AM_SKill_4")
        (`PrimitiveComponent.SetCollisionResponseToChannel` (`Character.CapsuleComponent` (`self.Hero`)) "ECC_Pawn" "ECR_Block")))
    (`self.K2_EndAbility`)
    (else
      (`self.K2_EndAbility`))))