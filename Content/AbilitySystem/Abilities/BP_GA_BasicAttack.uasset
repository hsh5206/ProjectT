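; Gameplay Ability for a hero's combo basic attack.
; The locally controlled hero calls ServerPlayMontage with an "Attack" section named from CurrentCombo, then stops the montage and ends the ability on the BasicAttackEnd event.
; In parallel, the authority waits for SmallHit events and applies GE_GetHit from the hero to the payload's target character, keeping hit effects server-side.
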(event `self.K2_ActivateAbility`
  (bind (_returnvalue_owneractor _returnvalue_avataractor) (break `GameplayAbilityActorInfo` (`self.GetActorInfo`)))
  (bind _asbase_hero (cast `BaseHero` _returnvalue_avataractor))
  (`|ExecutionSequence`
    (:`then_0`
      (if (`Pawn.IsLocallyControlled` _asbase_hero)
        (set `self.SectionName` (`KismetStringLibrary.Conv_StringToName` (`KismetStringLibrary.Concat_StrStr` "Attack" (`KismetStringLibrary.Conv_IntToString` (`BaseHero.CurrentCombo` _asbase_hero)))))
        (`BaseCharacter.ServerPlayMontage` _asbase_hero (`self.Montage to Play`) (`self.SectionName`))
        (`AbilityTask_WaitGameplayEvent.WaitGameplayEvent` (struct :`TagName` "Event.Attack.BasicAttackEnd") null
          (:`EventReceived`
            (`BaseCharacter.ServerStopMontage` _asbase_hero (`self.Montage to Play`))
            (`self.K2_EndAbility`)))))
    (:`then_1`
      (if (`Actor.HasAuthority` _asbase_hero)
        (bind (_asynctaskproxy _payload) (`AbilityTask_WaitGameplayEvent.WaitGameplayEvent` (struct :`TagName` "Event.Hit.SmallHit") null)
          (:`EventReceived`
            (bind _asbase_character (cast `BaseCharacter` (`.Target` (break `GameplayEventData` _payload))))
            (`AbilitySystemComponent.BP_ApplyGameplayEffectToTarget` (`AbilitySystemBlueprintLibrary.GetAbilitySystemComponent` _asbase_hero) "/Game/AbilitySystem/Effects/GE_GetHit.GE_GetHit_C" (`AbilitySystemBlueprintLibrary.GetAbilitySystemComponent` _asbase_character) 0.0 (make `GameplayEffectContextHandle`))))))))